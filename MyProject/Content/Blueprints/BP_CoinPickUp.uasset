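; Coin pickup that credits the Money actor found at BeginPlay, then respawns two seconds later with fire effects and a timeline-driven spin.
; PickUp shows the coin widget, advances a wrapping counter, hides the coin, plays a one-time explosion sound and saves any new high score.
; Christ restores visibility and collision with a brief fire sound.
; The construction script flattens the coin and scatters randomly scaled meshes around it.
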(event EventBeginPlay
  (bind _returnvalue (Actor|GetActorOfClass "/Game/Blueprints/Money.Money_C"))
  (Variables|Default|SetWallet _returnvalue))

(event EventTick
  (params (DeltaSeconds :type Float%20%28single-precision%29)))

(event Collision|EventActorBeginOverlap
  (params (OtherActor :type Actor%20Object%20Reference))
  (if (Utilities|NotCoinPickUpClass OtherActor)
    (CallFunction|PickUp)
    (Utilities|FlowControl|Delay 2.0)
    (CallFunction|Christ)
    (bind _returnvalue (Effects|SpawnEmitteratLocation "/Game/StarterContent/Particles/P_Fire.P_Fire" (Transformation|GetActorLocation)))
    (Utilities|FlowControl|Sequence
      (:then_0
        (bind _newtrack_0 (Timeline|Timeline Play)
          (:Update
            (Transformation|SetActorRotation (Math|Rotator|MakeRotator 0.0 0.0 _newtrack_0)))))
      (:then_1
        (Utilities|FlowControl|Delay 1.0)
        (Components|DestroyComponent _returnvalue)))))

(fn ConstructionScript
  (bind _returnvalue (Math|Random|RandomFloatinRange 0.05 0.5))
  (Transformation|SetRelativeScale3D (Variables|Default|GetSM_Coin) "1.000000,1.000000,0.250000")
  (for _index (range 0 6)
    (AddComponent|AddStaticMeshComponent false (Math|Transform|MakeTransform (Math|Vector|MakeVector (Math|Random|RandomFloatinRange -5e+01 5e+01) (Math|Random|RandomFloatinRange -5e+01 5e+01) (Math|Random|RandomFloatinRange 0.0 1e+02)) "0, 0, 0" (Math|Vector|MakeVector _returnvalue _returnvalue _returnvalue)))))

(fn PickUp
  (Utilities|FlowControl|Sequence
    (:then_0
      (Default|ShowYourself (Variables|/Game/Blueprints/Money.Money_C|GetCoinWidget (Variables|Default|GetWallet))))
    (:then_1
      (bind _result (Math|Integer|IncrementInt (Variables|/Game/Blueprints/Money.Money_C|GetNext (Variables|Default|GetWallet)))
        (:%20%20
          (if (> _result 6)
            (Variables|/Game/Blueprints/Money.Money_C|SetNext (Variables|Default|GetWallet) 0)))))
    (:then_2
      (Math|Integer|IncrementInt (Variables|/Game/Blueprints/Money.Money_C|GetMoney (Variables|Default|GetWallet))
        (:%20%20
          (Rendering|SetActorHiddenInGame true)
          (Collision|SetActorEnableCollision false)
          (Utilities|FlowControl|DoOnce false
            (:Completed
              (Audio|PlaySoundatLocation "/Game/StarterContent/Audio/Explosion02.Explosion02" (Transformation|GetActorLocation) "0, 0, 0" 1.0 1.0 0.0 0 0 0 0))))))
    (:then_3
      (bind _returnvalue (SaveGame|LoadGamefromSlot "HighScore"))
      (bind _assb_high_score_save (Utilities|Casting|CastToSB_HighScoreSave _returnvalue))
      (if (> (Variables|/Game/Blueprints/Money.Money_C|GetMoney (Variables|Default|GetWallet)) (Variables|/Game/Blueprints/SB_HighScoreSave.SB_HighScoreSave_C|GetHighScoreNumber _assb_high_score_save))
        (bind _returnvalue_2 (SaveGame|CreateSaveGameObject "/Game/Blueprints/SB_HighScoreSave.SB_HighScoreSave_C"))
        (Variables|/Game/Blueprints/SB_HighScoreSave.SB_HighScoreSave_C|SetHighScoreNumber _returnvalue_2 (Variables|/Game/Blueprints/Money.Money_C|GetMoney (Variables|Default|GetWallet)))
        (SaveGame|SaveGametoSlot _returnvalue_2 "HighScore")))))

(fn Christ
  (Rendering|SetActorHiddenInGame false)
  (Collision|SetActorEnableCollision true)
  (bind _returnvalue (Audio|SpawnSoundatLocation "/Game/StarterContent/Audio/Fire01.Fire01" (Transformation|GetActorLocation) "0, 0, 0" 1.0 1.0 0.0 0 0))
  (Audio|Components|Audio|StopDelayed _returnvalue 1.0))